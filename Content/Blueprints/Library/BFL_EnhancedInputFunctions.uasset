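; Blueprint function library that wraps Enhanced Input mapping context changes for the first local player.
; EasyAddMappingContext and EasyRemoveMappingContext validate player controller 0 and its Enhanced Input local player subsystem, then add or remove the given context.
; Adds always use priority zero, and both calls silently do nothing when the controller or subsystem is invalid.
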(fn `EasyAddMappingContext`
  (params (MappingContext :type "InputMappingContext Object Reference"))
  (bind _returnvalue (`GameplayStatics.GetPlayerController` null))
  (bind _returnvalue_2 (pcsubsystem `EnhancedInputLocalPlayerSubsystem` _returnvalue))
  (`/Engine/EditorBlueprintResources/StandardMacros.IsValid` _returnvalue
    (:`Is Valid`
      (`/Engine/EditorBlueprintResources/StandardMacros.IsValid` _returnvalue_2
        (:`Is Valid`
          (`EnhancedInputSubsystemInterface.AddMappingContext` _returnvalue_2 (`local.MappingContext`) 0 (struct)))))))

(fn `EasyRemoveMappingContext`
  (params (MappingContext :type "InputMappingContext Object Reference"))
  (bind _returnvalue (`GameplayStatics.GetPlayerController` null))
  (bind _returnvalue_2 (pcsubsystem `EnhancedInputLocalPlayerSubsystem` _returnvalue))
  (`/Engine/EditorBlueprintResources/StandardMacros.IsValid` _returnvalue
    (:`Is Valid`
      (`/Engine/EditorBlueprintResources/StandardMacros.IsValid` _returnvalue_2
        (:`Is Valid`
          (`EnhancedInputSubsystemInterface.RemoveMappingContext` _returnvalue_2 (`local.MappingContext`) (struct)))))))